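; Player pawn that slides left and right along the world X axis and spawns the ball actor when play begins.
; LeftRight axis input applies a fixed, swept offset per update, based only on the sign of the axis and not scaled by delta time.
; Spawn creates the ball at the capsule's transform, stores it as Play and binds an event to its Death dispatcher.
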(event `self.ReceiveActorBeginOverlap`
  (params (OtherActor :type "Actor Object Reference")))

(event `self.ReceiveBeginPlay`
  (`self.Spawn`))

(event `InputAxis|LeftRight`
  (params (AxisValue :type "Float (single-precision)"))
  (if (< AxisValue 0.0)
    (`self.K2_AddActorWorldOffset` (-5.0 0.0 0.0) true)))

(event `InputAxis|LeftRight`
  (params (AxisValue :type "Float (single-precision)"))
  (if (> AxisValue 0.0)
    (`self.K2_AddActorWorldOffset` (5.0 0.0 0.0) true)))

(fn `Spawn`
  (bind _returnvalue (`|SpawnActorFromClass` "/Game/NewContent/BP_Ball.BP_Ball_C" (`SceneComponent.K2_GetComponentToWorld` (`self.Capsule`)) "AlwaysSpawn" "OverrideRootScale" null null))
  (bind _output_get (set `self.Play` _returnvalue))
  (add `/Game/NewContent/BP_Ball.Death` _output_get (`|CreateDelegate` :!event `Spawn`))
  (return))

(fn `UserConstructionScript`)