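; BP_Ball is a bouncing ball actor that moves in a straight line and reflects off whatever blocks it.
; Each Tick it makes a swept offset move along Direction scaled by Speed and delta time, mirroring Direction about the impact normal on a blocking hit.
; Overlapping a KillZVolume calls Death and destroys the ball.
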(event `self.ReceiveActorBeginOverlap`
  (params (OtherActor :type "Actor Object Reference"))
  (cast `KillZVolume` OtherActor)
  (`self.Death`)
  (`self.K2_DestroyActor`))

(event `self.ReceiveTick`
  (params (DeltaSeconds :type "Float (single-precision)"))
  (bind _sweephitresult (`self.K2_AddActorWorldOffset` (* (* (`self.direction`) (`self.speed`)) DeltaSeconds) true))
  (bind (_bblockinghit _binitialoverlap _time _distance _location _impactpoint _normal _impactnormal _physmat _hitactor) (`GameplayStatics.BreakHitResult` _sweephitresult))
  (if _bblockinghit
    (set `self.direction` (`KismetMathLibrary.GetReflectionVector` (`self.direction`) _impactnormal))))

(fn `UserConstructionScript`)